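; BP_Main is an actor that spawns a BP_Sub and a BP_TheOther at opposite diagonal offsets from its own location when play begins.
; It stores a reference to each spawned actor and passes itself to BP_TheOther through BPMainRef, giving that actor a link back.
; Between the spawns it sets TestVarToWatch to a literal integer, and its construction script is empty.
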(event `self.ReceiveBeginPlay`
  (bind _returnvalue (`|SpawnActorFromClass` "/Game/BP_Sub.BP_Sub_C" (`KismetMathLibrary.MakeTransform` (+ (`self.K2_GetActorLocation`) (300.0 300.0 100.0))) "AlwaysSpawn" "OverrideRootScale" null null))
  (set `self.RefSub` _returnvalue)
  (set `self.TestVarToWatch` 0)
  (bind _returnvalue_2 (`|SpawnActorFromClass` "/Game/BP_TheOther.BP_TheOther_C" (`KismetMathLibrary.MakeTransform` (+ (`self.K2_GetActorLocation`) (-300.0 -300.0 100.0))) "AlwaysSpawn" "OverrideRootScale" null self null))
  (set `self.RefTheOther` _returnvalue_2))

(fn `UserConstructionScript`)